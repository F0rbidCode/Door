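; Multi-part door that opens and closes on alternate presses of Q, via an event bound on the player character.
; Opening chains three timelines: the sphere rotates, two panels slide apart, then two more move in opposite vertical directions.
; Closing runs separate timelines backwards in reverse order, each seeded from its forward twin's playback position.
; Updates lerp from transforms cached at BeginPlay to composed end offsets, mirrored for each second panel.
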(event Custom|OnQPressed%20Handler
  ;[1 1 1] Oppen And Close the door
  (Utilities|FlowControl|FlipFlop
    (:A
      ;;[1 0.7648 0.5141] Get the position of the reverse timeline and set it to the time of this timeline
      (Components|Timeline|SetNewTime (Variables|Default|GetRotation%20Timeline) (Components|Timeline|GetPlaybackPosition (Variables|Default|GetReverse%20Rotation%20Timeline)))
      ;;[1 0.7005 0.5586] First rotate the Sphere, Use lerp and a timeline to smoothly transition between the start and end positions
      (bind _doorrotation (Timeline|Rotation%20Timeline Play)
        (:Update
          (Transformation|SetRelativeRotation (Variables|Default|GetShape_Sphere) (Math|Rotator|Lerp(Rotator) (Variables|Default|GetInitial%20rotation) (Variables|Default|GetEnd%20Rotation) _doorrotation) false false))
        (:Finished
          ;;[1 0.7676 0.7377] Get the position of the reverse timeline and set it to the time of this timeline
          (Components|Timeline|SetNewTime (Variables|Default|GetSliding%20Timeline) (Components|Timeline|GetPlaybackPosition (Variables|Default|GetReverse%20Sliding%20Timeline)))
          ;;[1 0.778 0.7481] Slide both sections of the door appart, using a singe timeline to do both doors and lerp to smoothly transition beteen the start and end positions
          (bind _sliding_timeline (Timeline|Sliding%20Timeline Play)
            (:Update
              (Transformation|SetRelativeTransform (Variables|Default|GetShape_Cube) (Math|Transform|Lerp(Transform) (Variables|Default|GetSlidingDoor0%20Initial%20Position) (Math|Transform|ComposeTransforms (Variables|Default|GetSlidingDoor%20End%20position) (Variables|Default|GetSlidingDoor0%20Initial%20Position)) _sliding_timeline) false false)
              (Transformation|SetRelativeTransform (Variables|Default|GetShape_Cube1) (Math|Transform|Lerp(Transform) (Variables|Default|GetSlidingDoor1%20Initial%20Position) (Math|Transform|ComposeTransforms (Variables|Default|GetSlidingDoor1%20Initial%20Position) (Math|Conversions|ToTransform(Vector) (* (.location (Variables|Default|GetSlidingDoor%20End%20position)) "-1.000000,0.000000,0.000000"))) _sliding_timeline) false false))
            (:Finished
              ;;[1 0.7676 0.7377] Get the position of the reverse timeline and set it to the time of this timeline
              (Components|Timeline|SetNewTime (Variables|Default|GetLifting%20Door%20Timeline) (Components|Timeline|GetPlaybackPosition (Variables|Default|GetReverse%20Lifting%20Timeline)))
              ;;[1 0.778 0.7481] Lift and lower both sections of the door appart, using a singe timeline to do both doors and lerp to smoothly transition beteen the start and end positions
              (bind _sliding_timeline_2 (Timeline|Lifting%20Door%20Timeline Play)
                (:Update
                  (Transformation|SetRelativeTransform (Variables|Default|GetShape_Cube2) (Math|Transform|Lerp(Transform) (Variables|Default|GetLiftingDoor%202%20initial%20Position) (Math|Transform|ComposeTransforms (Variables|Default|GetLiftingDoor%20End%20Position) (Variables|Default|GetLiftingDoor%202%20initial%20Position)) _sliding_timeline_2) false false)
                  (Transformation|SetRelativeTransform (Variables|Default|GetShape_Cube3) (Math|Transform|Lerp(Transform) (Variables|Default|GetLiftingDoor%203%20initial%20Position) (Math|Transform|ComposeTransforms (Variables|Default|GetLiftingDoor%203%20initial%20Position) (Math|Conversions|ToTransform(Vector) (* (.location (Variables|Default|GetLiftingDoor%20End%20Position)) "-1.000000,0.000000,-1.000000"))) _sliding_timeline_2) false false))))))))
    (:B
      ;;[1 0.7676 0.7377] Get the position of the Forward timeline and set it to the time of this timeline
      (Components|Timeline|SetNewTime (Variables|Default|GetReverse%20Lifting%20Timeline) (Components|Timeline|GetPlaybackPosition (Variables|Default|GetLifting%20Door%20Timeline)))
      ;;[1 0.778 0.7481] Lift and lower both sections of the door appart, using a singe timeline to do both doors and lerp to smoothly transition beteen the start and end positions
      (bind _sliding_timeline_3 (Timeline|Reverse%20Lifting%20Timeline Reverse)
        (:Update
          (Transformation|SetRelativeTransform (Variables|Default|GetShape_Cube2) (Math|Transform|Lerp(Transform) (Variables|Default|GetLiftingDoor%202%20initial%20Position) (Math|Transform|ComposeTransforms (Variables|Default|GetLiftingDoor%20End%20Position) (Variables|Default|GetLiftingDoor%202%20initial%20Position)) _sliding_timeline_3) false false)
          (Transformation|SetRelativeTransform (Variables|Default|GetShape_Cube3) (Math|Transform|Lerp(Transform) (Variables|Default|GetLiftingDoor%203%20initial%20Position) (Math|Transform|ComposeTransforms (Variables|Default|GetLiftingDoor%203%20initial%20Position) (Math|Conversions|ToTransform(Vector) (* (.location (Variables|Default|GetLiftingDoor%20End%20Position)) "-1.000000,0.000000,-1.000000"))) _sliding_timeline_3) false false))
        (:Finished
          ;;[1 0.8151 0.765] Get The position of the forward timeline and set it to the time of this timeline
          (Components|Timeline|SetNewTime (Variables|Default|GetReverse%20Sliding%20Timeline) (Components|Timeline|GetPlaybackPosition (Variables|Default|GetSliding%20Timeline)))
          ;;[1 0.778 0.7481] Slide both sections of the door appart, using a singe timeline to do both doors and lerp to smoothly transition beteen the start and end positions
          (bind _sliding_timeline_4 (Timeline|Reverse%20Sliding%20Timeline Reverse)
            (:Update
              (Transformation|SetRelativeTransform (Variables|Default|GetShape_Cube) (Math|Transform|Lerp(Transform) (Variables|Default|GetSlidingDoor0%20Initial%20Position) (Math|Transform|ComposeTransforms (Variables|Default|GetSlidingDoor%20End%20position) (Variables|Default|GetSlidingDoor0%20Initial%20Position)) _sliding_timeline_4) false false)
              (Transformation|SetRelativeTransform (Variables|Default|GetShape_Cube1) (Math|Transform|Lerp(Transform) (Variables|Default|GetSlidingDoor1%20Initial%20Position) (Math|Transform|ComposeTransforms (Variables|Default|GetSlidingDoor1%20Initial%20Position) (Math|Conversions|ToTransform(Vector) (* (.location (Variables|Default|GetSlidingDoor%20End%20position)) "-1.000000,0.000000,0.000000"))) _sliding_timeline_4) false false))
            (:Finished
              ;;[1 0.7648 0.5141] Get the position of the forward timeline and set it to the time of this timeline
              (Components|Timeline|SetNewTime (Variables|Default|GetReverse%20Rotation%20Timeline) (Components|Timeline|GetPlaybackPosition (Variables|Default|GetRotation%20Timeline)))
              ;;[1 0.7005 0.5586] First rotate the Sphere, Use lerp and a timeline to smoothly transition between the start and end positions
              (bind _doorrotation_2 (Timeline|Reverse%20Rotation%20Timeline Reverse)
                (:Update
                  (Transformation|SetRelativeRotation (Variables|Default|GetShape_Sphere) (Math|Rotator|Lerp(Rotator) (Variables|Default|GetInitial%20rotation) (Variables|Default|GetEnd%20Rotation) _doorrotation_2) false false))
                (:Finished)))))))))

(event EventBeginPlay
  (Utilities|FlowControl|Sequence
    (:then_0
      ;[1 1 1] Get the Player character
      (bind _outactors (Actor|GetAllActorsOfClass "/Game/ThirdPerson/Blueprints/BP_ThirdPersonCharacter.BP_ThirdPersonCharacter_C"))
      (Variables|Default|Setplayer (Utilities|Array|Get(acopy) _outactors)))
    (:then_1
      ;[1 1 1] Bind the players OnQPressed event to the OnQPressed Handler
      (EventDispatchers|BindEventtoOnQPressed (Variables|Default|Getplayer) (delegate Custom|OnQPressed%20Handler)))
    (:then_2
      ;[1 1 1] Get Door Location and Rotations
      (Variables|Default|SetSlidingDoor0%20Initial%20Position (Transformation|GetRelativeTransform (Variables|Default|GetShape_Cube)))
      (Variables|Default|SetSlidingDoor1%20Initial%20Position (Transformation|GetRelativeTransform (Variables|Default|GetShape_Cube1)))
      (Variables|Default|SetInitial%20rotation (Transformation|GetWorldRotation (Variables|Default|GetShape_Sphere)))
      (Variables|Default|SetLiftingDoor%202%20initial%20Position (Transformation|GetRelativeTransform (Variables|Default|GetShape_Cube2)))
      (Variables|Default|SetLiftingDoor%203%20initial%20Position (Transformation|GetRelativeTransform (Variables|Default|GetShape_Cube3))))))

(fn ConstructionScript)