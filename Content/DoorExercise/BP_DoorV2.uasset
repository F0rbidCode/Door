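; Multi-stage door actor that opens and closes on alternate presses of Q, via the player character's OnQPressed event.
; Opening chains three timelines through their Finished events: rotate the sphere, slide two panels apart, then lift the other pair; closing reverses them in opposite order.
; Each press stops all timelines before changing direction.
; Panels lerp from transforms cached at BeginPlay to composed end offsets, with one shared offset mirrored per pair.
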(event Custom|OnQPressed%20Handler
  ;[1 1 1] Oppen And Close the door
  (Utilities|FlowControl|FlipFlop
    (:A
      (Variables|Revised|SetOpening true))
    (:B
      (Variables|Revised|SetOpening false)))
  (CallFunction|StopTimelines)
  (if (Variables|Revised|GetOpening)
    (CallFunction|Rotate)
    (else
      (CallFunction|ReverseLift))))

(event Custom|Lift
  ;[1 1 1] Oppen And Close the door
  ;;[1 0.778 0.7481] Lift and lower both sections of the door appart, using a singe timeline to do both doors and lerp to smoothly transition beteen the start and end positions
  (bind _sliding_timeline (Timeline|Lifting%20Door%20Timeline Play)
    (:Update
      (Transformation|SetRelativeTransform (Variables|Default|GetShape_Cube2) (Math|Transform|Lerp(Transform) (Variables|Default|GetLiftingDoor%202%20initial%20Position) (Math|Transform|ComposeTransforms (Variables|Default|GetLiftingDoor%20End%20Position) (Variables|Default|GetLiftingDoor%202%20initial%20Position)) _sliding_timeline) false false)
      (Transformation|SetRelativeTransform (Variables|Default|GetShape_Cube3) (Math|Transform|Lerp(Transform) (Variables|Default|GetLiftingDoor%203%20initial%20Position) (Math|Transform|ComposeTransforms (Variables|Default|GetLiftingDoor%203%20initial%20Position) (Math|Conversions|ToTransform(Vector) (* (.location (Variables|Default|GetLiftingDoor%20End%20Position)) "-1.000000,0.000000,-1.000000"))) _sliding_timeline) false false))
    (:Finished
      (if (not (Variables|Revised|GetOpening))
        (CallFunction|ReverseSlide)))))

(event Custom|Rotate
  ;[1 1 1] Oppen And Close the door
  ;;[1 0.7005 0.5586] First rotate the Sphere, Use lerp and a timeline to smoothly transition between the start and end positions
  (bind _doorrotation (Timeline|Rotation%20Timeline Play)
    (:Update
      (Transformation|SetRelativeRotation (Variables|Default|GetShape_Sphere) (Math|Rotator|Lerp(Rotator) (Variables|Default|GetInitial%20rotation) (Variables|Default|GetEnd%20Rotation) _doorrotation) false false))
    (:Finished
      (if (Variables|Revised|GetOpening)
        (CallFunction|Slide)))))

(event Custom|ReverseRotate
  ;[1 1 1] Oppen And Close the door
  ;;[1 0.7005 0.5586] First rotate the Sphere, Use lerp and a timeline to smoothly transition between the start and end positions
  (bind _doorrotation (Timeline|Rotation%20Timeline Reverse)
    (:Update
      (Transformation|SetRelativeRotation (Variables|Default|GetShape_Sphere) (Math|Rotator|Lerp(Rotator) (Variables|Default|GetInitial%20rotation) (Variables|Default|GetEnd%20Rotation) _doorrotation) false false))
    (:Finished
      (if (Variables|Revised|GetOpening)
        (CallFunction|Slide)))))

(event Custom|ReverseLift
  ;[1 1 1] Oppen And Close the door
  ;;[1 0.778 0.7481] Lift and lower both sections of the door appart, using a singe timeline to do both doors and lerp to smoothly transition beteen the start and end positions
  (bind _sliding_timeline (Timeline|Lifting%20Door%20Timeline Reverse)
    (:Update
      (Transformation|SetRelativeTransform (Variables|Default|GetShape_Cube2) (Math|Transform|Lerp(Transform) (Variables|Default|GetLiftingDoor%202%20initial%20Position) (Math|Transform|ComposeTransforms (Variables|Default|GetLiftingDoor%20End%20Position) (Variables|Default|GetLiftingDoor%202%20initial%20Position)) _sliding_timeline) false false)
      (Transformation|SetRelativeTransform (Variables|Default|GetShape_Cube3) (Math|Transform|Lerp(Transform) (Variables|Default|GetLiftingDoor%203%20initial%20Position) (Math|Transform|ComposeTransforms (Variables|Default|GetLiftingDoor%203%20initial%20Position) (Math|Conversions|ToTransform(Vector) (* (.location (Variables|Default|GetLiftingDoor%20End%20Position)) "-1.000000,0.000000,-1.000000"))) _sliding_timeline) false false))
    (:Finished
      (if (not (Variables|Revised|GetOpening))
        (CallFunction|ReverseSlide)))))

(event Custom|Slide
  ;[1 1 1] Oppen And Close the door
  ;;[1 0.778 0.7481] Slide both sections of the door appart, using a singe timeline to do both doors and lerp to smoothly transition beteen the start and end positions
  (bind _sliding_timeline (Timeline|Sliding%20Timeline Play)
    (:Update
      (Transformation|SetRelativeTransform (Variables|Default|GetShape_Cube) (Math|Transform|Lerp(Transform) (Variables|Default|GetSlidingDoor0%20Initial%20Position) (Math|Transform|ComposeTransforms (Variables|Default|GetSlidingDoor%20End%20position) (Variables|Default|GetSlidingDoor0%20Initial%20Position)) _sliding_timeline) false false)
      (Transformation|SetRelativeTransform (Variables|Default|GetShape_Cube1) (Math|Transform|Lerp(Transform) (Variables|Default|GetSlidingDoor1%20Initial%20Position) (Math|Transform|ComposeTransforms (Variables|Default|GetSlidingDoor1%20Initial%20Position) (Math|Conversions|ToTransform(Vector) (* (.location (Variables|Default|GetSlidingDoor%20End%20position)) "-1.000000,0.000000,0.000000"))) _sliding_timeline) false false))
    (:Finished
      (if (Variables|Revised|GetOpening)
        (CallFunction|Lift)
        (else
          (CallFunction|ReverseRotate))))))

(event Custom|ReverseSlide
  ;[1 1 1] Oppen And Close the door
  ;;[1 0.778 0.7481] Slide both sections of the door appart, using a singe timeline to do both doors and lerp to smoothly transition beteen the start and end positions
  (bind _sliding_timeline (Timeline|Sliding%20Timeline Reverse)
    (:Update
      (Transformation|SetRelativeTransform (Variables|Default|GetShape_Cube) (Math|Transform|Lerp(Transform) (Variables|Default|GetSlidingDoor0%20Initial%20Position) (Math|Transform|ComposeTransforms (Variables|Default|GetSlidingDoor%20End%20position) (Variables|Default|GetSlidingDoor0%20Initial%20Position)) _sliding_timeline) false false)
      (Transformation|SetRelativeTransform (Variables|Default|GetShape_Cube1) (Math|Transform|Lerp(Transform) (Variables|Default|GetSlidingDoor1%20Initial%20Position) (Math|Transform|ComposeTransforms (Variables|Default|GetSlidingDoor1%20Initial%20Position) (Math|Conversions|ToTransform(Vector) (* (.location (Variables|Default|GetSlidingDoor%20End%20position)) "-1.000000,0.000000,0.000000"))) _sliding_timeline) false false))
    (:Finished
      (if (Variables|Revised|GetOpening)
        (CallFunction|Lift)
        (else
          (CallFunction|ReverseRotate))))))

(event EventBeginPlay
  (Utilities|FlowControl|Sequence
    (:then_0
      ;[1 1 1] Get the Player character
      (bind _outactors (Actor|GetAllActorsOfClass "/Game/ThirdPerson/Blueprints/BP_ThirdPersonCharacter.BP_ThirdPersonCharacter_C"))
      (Variables|Default|Setplayer (Utilities|Array|Get(acopy) _outactors)))
    (:then_1
      ;[1 1 1] Bind the players OnQPressed event to the OnQPressed Handler
      (EventDispatchers|BindEventtoOnQPressed (Variables|Default|Getplayer) (EventDispatchers|CreateEvent :!event Custom|OnQPressed%20Handler)))
    (:then_2
      ;[1 1 1] Get Door Location and Rotations
      (Variables|Default|SetSlidingDoor0%20Initial%20Position (Transformation|GetRelativeTransform (Variables|Default|GetShape_Cube)))
      (Variables|Default|SetSlidingDoor1%20Initial%20Position (Transformation|GetRelativeTransform (Variables|Default|GetShape_Cube1)))
      (Variables|Default|SetInitial%20rotation (Transformation|GetWorldRotation (Variables|Default|GetShape_Sphere)))
      (Variables|Default|SetLiftingDoor%202%20initial%20Position (Transformation|GetRelativeTransform (Variables|Default|GetShape_Cube2)))
      (Variables|Default|SetLiftingDoor%203%20initial%20Position (Transformation|GetRelativeTransform (Variables|Default|GetShape_Cube3))))))

(fn ConstructionScript)

(fn StopTimelines
  (Audio|Components|Audio|Stop (Variables|Default|GetRotation%20Timeline))
  (return))